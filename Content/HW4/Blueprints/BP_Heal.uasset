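; BP_Heal is a heart-shaped health pickup that restores one point of health to an overlapping actor.
; On sphere overlap it calls Heal on that actor's HealthComponent, fetched without a validity check, then hides itself.
; Hiding turns off the heart's visibility and the sphere's collision instead of destroying the actor.
; The Reset event re-shows the heart and restores query-only collision, so the pickup can be reused.
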(event OnComponentBeginOverlap(Sphere)
  (params (OverlappedComponent :type Primitive%20Component%20Object%20Reference) (OtherActor :type Actor%20Object%20Reference) (OtherComp :type Primitive%20Component%20Object%20Reference) (OtherBodyIndex :type Integer) (bFromSweep :type Boolean) (SweepResult :type Hit%20Result%20Structure%20%28by%20ref%29))
  (bind _output_get (Variables|Default|SetHealthComponent (Actor|GetComponentbyClass OtherActor "/Game/HW4/Components/HealthComponent.HealthComponent_C")))
  (Default|Heal _output_get 1)
  (CallFunction|HideActor))

(event EventReset
  (CallFunction|ShowActor))

(fn ConstructionScript)

(fn HideActor
  (Collision|SetCollisionEnabled (Variables|Default|GetSphere) "NoCollision")
  (Rendering|SetVisibility (Variables|Default|GetHeart) false false))

(fn ShowActor
  (Rendering|SetVisibility (Variables|Default|GetHeart) true false)
  (Collision|SetCollisionEnabled (Variables|Default|GetSphere) "QueryOnly"))