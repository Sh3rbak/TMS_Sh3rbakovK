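; BP_Hammer is a hammer hazard that damages actors entering its box trigger and knocks the player away.
; On overlap, the player character is launched against its horizontal velocity with a fixed upward boost that overrides vertical speed.
; Every overlapping actor, player or not, then has its HealthComponent looked up and damaged, with no check that the component exists.
; An unconnected copy of this logic remains in the event graph.
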(event OnComponentBeginOverlap(Box)
  (params (OverlappedComponent :type Primitive%20Component%20Object%20Reference) (OtherActor :type Actor%20Object%20Reference) (OtherComp :type Primitive%20Component%20Object%20Reference) (OtherBodyIndex :type Integer) (bFromSweep :type Boolean) (SweepResult :type Hit%20Result%20Structure%20%28by%20ref%29))
  (bind _returnvalue (Game|GetPlayerCharacter 0))
  (Utilities|FlowControl|Sequence
    (:then_0
      (if (== OtherActor _returnvalue)
        (CallFunction|PushActorAway _returnvalue)))
    (:then_1
      (CallFunction|GetComponentHealth OtherActor))))

(fn ConstructionScript)

(fn GetComponentHealth
  (params (Target :type Actor%20Object%20Reference))
  (bind _output_get (Variables|Default|SetHealthComponent (Actor|GetComponentbyClass Target "/Game/HW4/Components/HealthComponent.HealthComponent_C")))
  (Default|TakeDamage _output_get 1)
  (return))

(fn PushActorAway
  (params (Target :type Character%20Object%20Reference))
  (bind _returnvalue (Transformation|GetVelocity Target))
  (Character|LaunchCharacter Target (Math|Vector|MakeVector (* (.x _returnvalue) -2.5) (* (.y _returnvalue) -2.5) 7.5e+02) false true)
  (return))