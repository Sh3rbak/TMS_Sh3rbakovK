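; BP_KillZone is a box trigger that penalizes any overlapping actor and sends it back to its checkpoint.
; On overlap it applies one point of damage through the actor's HealthComponent, without a validity check.
; It then validates the actor's CheckpointComponent, resolves the stored checkpoint to a transform via CheckpointFun, and teleports the actor there without sweeping.
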(event OnComponentBeginOverlap(Box)
  (params (OverlappedComponent :type Primitive%20Component%20Object%20Reference) (OtherActor :type Actor%20Object%20Reference) (OtherComp :type Primitive%20Component%20Object%20Reference) (OtherBodyIndex :type Integer) (bFromSweep :type Boolean) (SweepResult :type Hit%20Result%20Structure%20%28by%20ref%29))
  (CallFunction|GetComponentHealth OtherActor)
  (bind (_currectactor _transformcheckpoint) (CallFunction|GetCheckpointComponent OtherActor))
  (Transformation|SetActorTransform _currectactor _transformcheckpoint false true))

(fn ConstructionScript)

(fn GetCheckpointComponent
  (params (Actor :type Actor%20Object%20Reference))
  (bind _returnvalue (Actor|GetComponentbyClass Actor "/Game/HW4/Components/CheckpointComponent.CheckpointComponent_C"))
  (Utilities|IsValid _returnvalue
    (:Is%20Valid
      (bind _output_get (Variables|Default|SetCheckpoint _returnvalue))
      (bind _output_checpoint (Default|CheckpointFun _output_get (Variables|/Game/HW4/Components/CheckpointComponent.CheckpointComponent_C|GetChecpoint _output_get)))
      (return Actor _output_checpoint))))

(fn GetComponentHealth
  (params (Target :type Actor%20Object%20Reference))
  (bind _output_get (Variables|Default|SetHealthComponent (Actor|GetComponentbyClass Target "/Game/HW4/Components/HealthComponent.HealthComponent_C")))
  (Default|TakeDamage _output_get 1)
  (return))