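; BP_Obstacle is a spinning obstacle that knocks the player character away on contact.
; Tick continuously yaws the Obstacle component, and overlaps on Box and Box1 launch the player with velocity overrides, each using its own Arrow as the axis.
; GetReboundDirection uses 2D vector projection to find the closest point on that axis, then returns a fixed-strength push perpendicularly away from it with slight lift.
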(event OnComponentBeginOverlap(Box)
  (params (OverlappedComponent :type Primitive%20Component%20Object%20Reference) (OtherActor :type Actor%20Object%20Reference) (OtherComp :type Primitive%20Component%20Object%20Reference) (OtherBodyIndex :type Integer) (bFromSweep :type Boolean) (SweepResult :type Hit%20Result%20Structure%20%28by%20ref%29))
  (bind _returnvalue (Game|GetPlayerCharacter 0))
  (if (== OtherActor _returnvalue)
    (Character|LaunchCharacter _returnvalue (CallFunction|GetReboundDirection _returnvalue self (Variables|Default|GetArrow)) true true)))

(event OnComponentBeginOverlap(Box1)
  (params (OverlappedComponent :type Primitive%20Component%20Object%20Reference) (OtherActor :type Actor%20Object%20Reference) (OtherComp :type Primitive%20Component%20Object%20Reference) (OtherBodyIndex :type Integer) (bFromSweep :type Boolean) (SweepResult :type Hit%20Result%20Structure%20%28by%20ref%29))
  (bind _returnvalue (Game|GetPlayerCharacter 0))
  (if (== OtherActor _returnvalue)
    (Character|LaunchCharacter _returnvalue (CallFunction|GetReboundDirection _returnvalue self (Variables|Default|GetArrow1)) true true)))

(event EventTick
  (params (DeltaSeconds :type Float%20%28single-precision%29))
  (Transformation|AddLocalRotation (Variables|Default|GetObstacle) (Math|Rotator|MakeRotator 0.0 0.0 (* DeltaSeconds 4e+01)) false false))

(fn ConstructionScript)

(fn GetReboundDirection
  (params (Actor :type Actor%20Object%20Reference) (SelfActor :type Actor%20Object%20Reference) (Arrow :type Scene%20Component%20Object%20Reference))
  (bind _returnvalue (Transformation|GetActorLocation SelfActor))
  (bind _returnvalue_2 (Transformation|GetActorLocation Actor))
  (bind _returnvalue_3 (Math|Vector|GetForwardVector Arrow))
  (bind _returnvalue_4 (Math|Conversions|ToVector2D(Vector) _returnvalue))
  (bind _returnvalue_5 (Math|Conversions|ToVector2D(Vector) _returnvalue_2))
  (bind _returnvalue_6 (Math|Conversions|ToVector2D(Vector) _returnvalue_3))
  (bind _returnvalue_7 (Math|Vector2D|DotProduct(2D) _returnvalue_6 _returnvalue_6))
  (bind _returnvalue_8 (- _returnvalue_5 _returnvalue_4))
  (bind _returnvalue_9 (Math|Vector2D|DotProduct(2D) _returnvalue_8 _returnvalue_6))
  (bind _returnvalue_10 (/ _returnvalue_9 _returnvalue_7))
  (bind _returnvalue_11 (* _returnvalue_6 _returnvalue_10))
  (bind _returnvalue_12 (+ _returnvalue_4 _returnvalue_11))
  (bind _returnvalue_13 (- _returnvalue_12 _returnvalue_5))
  (bind _returnvalue_14 (Class|KismetMathLibrary|NormalSafe2D _returnvalue_13 0.0))
  (bind _returnvalue_15 (* _returnvalue_14 -1.0))
  (bind _returnvalue_16 (* _returnvalue_15 5e+02))
  (return (Math|Vector|MakeVector (.x _returnvalue_16) (.y _returnvalue_16) 1e+01)))