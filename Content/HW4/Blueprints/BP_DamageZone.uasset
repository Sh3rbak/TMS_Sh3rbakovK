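; BP_DamageZone is a damage-over-time area that hurts an actor through its HealthComponent.
; Box begin overlap stores the other actor's HealthComponent and starts a looping one-second timer that calls TakeDamage on it.
; Any actor starts the timer, with no validity check, overwriting the single stored component and handle.
; End overlap clears the current timer only when player character 0 leaves.
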(event OnComponentBeginOverlap(Box)
  (params (OverlappedComponent :type Primitive%20Component%20Object%20Reference) (OtherActor :type Actor%20Object%20Reference) (OtherComp :type Primitive%20Component%20Object%20Reference) (OtherBodyIndex :type Integer) (bFromSweep :type Boolean) (SweepResult :type Hit%20Result%20Structure%20%28by%20ref%29))
  (Variables|Default|SetHealthComponent (Actor|GetComponentbyClass OtherActor "/Game/HW4/Components/HealthComponent.HealthComponent_C"))
  (bind _returnvalue (Utilities|Time|SetTimerbyEvent (delegate Custom|TakeDamageEvent) 1.0 true))
  (Variables|Default|SetDamageTimer _returnvalue))

(event OnComponentEndOverlap(Box)
  (params (OverlappedComponent :type Primitive%20Component%20Object%20Reference) (OtherActor :type Actor%20Object%20Reference) (OtherComp :type Primitive%20Component%20Object%20Reference) (OtherBodyIndex :type Integer))
  (if (== OtherActor (Game|GetPlayerCharacter 0))
    (Utilities|Time|ClearandInvalidateTimerbyHandle (Variables|Default|GetDamageTimer))))

(event Custom|TakeDamageEvent
  (Default|TakeDamage (Variables|Default|GetHealthComponent) 1))

(fn ConstructionScript)