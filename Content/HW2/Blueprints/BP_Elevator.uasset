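; BP_Elevator is an elevator that alternates between up and down when triggered by overlaps on its capsule.
; Begin overlap passes a DoOnce gate, which resets when the player pawn leaves.
; After a short delay, a player check and IsUp flag choose whether the MovementElevator timeline plays or reverses, moving the SMObstacle8001 component's relative location.
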(event OnComponentBeginOverlap(Capsule)
  (params (OverlappedComponent :type Primitive%20Component%20Object%20Reference) (OtherActor :type Actor%20Object%20Reference) (OtherComp :type Primitive%20Component%20Object%20Reference) (OtherBodyIndex :type Integer) (bFromSweep :type Boolean) (SweepResult :type Hit%20Result%20Structure%20%28by%20ref%29))
  (Utilities|FlowControl|DoOnce false
    (:Completed
      (Utilities|FlowControl|Delay 0.5)
      (if (and (== OtherActor (Game|Player|GetPlayerPawn 0)) (not (Variables|Default|GetIsUp)))
        (Variables|Default|SetIsUp true)
        (bind _movement (Timeline|MovementElevator Play)
          (:Update
            (Transformation|SetRelativeLocation (Variables|Default|GetSM_obstacle_8_001) _movement false false)))
        (else
          (Variables|Default|SetIsUp false)
          (Timeline|MovementElevator Reverse))))))

(event OnComponentEndOverlap(Capsule)
  (params (OverlappedComponent :type Primitive%20Component%20Object%20Reference) (OtherActor :type Actor%20Object%20Reference) (OtherComp :type Primitive%20Component%20Object%20Reference) (OtherBodyIndex :type Integer))
  (if (== OtherActor (Game|Player|GetPlayerPawn 0))
    (Utilities|FlowControl|DoOnce false) ; enters at Reset
  ))

(fn ConstructionScript)