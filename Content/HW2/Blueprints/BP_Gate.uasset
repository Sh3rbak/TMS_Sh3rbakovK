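; Gate actor that swings open while the player pawn stands in its box trigger and closes when the pawn leaves.
; Box overlap events set IsOpen and play or reverse RotateTimeLine, which lerps the Scene component's relative pitch.
; Each timeline update also calls TernOnLights, showing two spotlights when IsOpen is true and hiding them as soon as closing starts.
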(event OnComponentBeginOverlap(Box)
  (params (OverlappedComponent :type Primitive%20Component%20Object%20Reference) (OtherActor :type Actor%20Object%20Reference) (OtherComp :type Primitive%20Component%20Object%20Reference) (OtherBodyIndex :type Integer) (bFromSweep :type Boolean) (SweepResult :type Hit%20Result%20Structure%20%28by%20ref%29))
  (if (and (== OtherActor (Game|Player|GetPlayerPawn 0)) (not (Variables|Default|GetIsOpen)))
    (Variables|Default|SetIsOpen true)
    (bind _rotate_door (Timeline|RotateTimeLine Play)
      (:Update
        (Transformation|SetRelativeRotation (Variables|Default|GetScene) (Math|Rotator|MakeRotator 0.0 (Math|Float|Lerp -5e+01 0.0 _rotate_door) 0.0) false false)
        (CallFunction|TernonLights (Variables|Default|GetIsOpen))))))

(event OnComponentEndOverlap(Box)
  (params (OverlappedComponent :type Primitive%20Component%20Object%20Reference) (OtherActor :type Actor%20Object%20Reference) (OtherComp :type Primitive%20Component%20Object%20Reference) (OtherBodyIndex :type Integer))
  (if (and (== OtherActor (Game|Player|GetPlayerPawn 0)) (Variables|Default|GetIsOpen))
    (Variables|Default|SetIsOpen false)
    (bind _rotate_door (Timeline|RotateTimeLine Reverse)
      (:Update
        (Transformation|SetRelativeRotation (Variables|Default|GetScene) (Math|Rotator|MakeRotator 0.0 (Math|Float|Lerp -5e+01 0.0 _rotate_door) 0.0) false false)
        (CallFunction|TernonLights (Variables|Default|GetIsOpen))))))

(fn ConstructionScript)

(fn TernonLights
  (params (Is%20open :type Boolean))
  (bind _spotlight (Variables|Default|GetSpotLight))
  (bind _spotlight1 (Variables|Default|GetSpotLight1))
  (if Is%20open
    (Rendering|SetVisibility _spotlight true false)
    (Rendering|SetVisibility _spotlight1 true false)
    (else
      (Rendering|SetVisibility _spotlight false false)
      (Rendering|SetVisibility _spotlight1 false false))))