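; BP_Dynamite is a hazard actor that penalizes the HW3 third-person character when it overlaps it.
; On overlap it subtracts Damage from the character's CoinCollectorComponent and launches it upward and against its horizontal velocity, with uneven X and Y scaling.
; It then hides its mesh and disables capsule collision rather than destroying itself, so the Reset event can restore both.
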(event Collision|EventActorBeginOverlap
  (params (OtherActor :type Actor%20Object%20Reference))
  (bind _asbp_hw3_third_person_character (Utilities|Casting|CastToBP_HW3_ThirdPersonCharacter OtherActor))
  (Default|AddCoins (Variables|/Game/HW3/Blueprints/Framefork/BP_HW3_ThirdPersonCharacter.BP_HW3_ThirdPersonCharacter_C|GetCoinCollectorComponent _asbp_hw3_third_person_character) (* (Variables|Default|GetDamage) -1))
  (Character|LaunchCharacter _asbp_hw3_third_person_character (Math|Vector|MakeVector (* (.x (Transformation|GetVelocity _asbp_hw3_third_person_character)) -5.0) (* (.y (Transformation|GetVelocity _asbp_hw3_third_person_character)) -2.5) 1e+03) true true)
  (Rendering|SetVisibility (Variables|Default|GetStaticMesh) false false)
  (Collision|SetCollisionEnabled (Variables|Default|GetCapsule) "NoCollision"))

(event EventReset
  (Rendering|SetVisibility (Variables|Default|GetStaticMesh) true false)
  (Collision|SetCollisionEnabled (Variables|Default|GetCapsule) "QueryOnly"))

(fn ConstructionScript)