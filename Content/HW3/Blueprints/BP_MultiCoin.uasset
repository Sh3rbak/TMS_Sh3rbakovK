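; BP_MultiCoin is a coin pickup worth a configurable number of coins.
; On overlap it adds NumberOfCoins to the overlapping actor's CoinCollectorComponent, with no validity check on that component.
; It then disables Sphere collision and hides the mesh instead of destroying itself, so the Reset event can restore query collision and visibility.
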(event Collision|EventActorBeginOverlap
  (params (OtherActor :type Actor%20Object%20Reference))
  (Default|AddCoins (Actor|GetComponentbyClass OtherActor "/Game/HW3/Components/CoinCollectorComponent.CoinCollectorComponent_C") (Variables|Default|GetNumberOfCoins))
  (Collision|SetCollisionEnabled (Variables|Default|GetSphere) "NoCollision")
  (Rendering|SetVisibility (Variables|Default|GetStaticMesh) false false))

(event EventReset
  (Collision|SetCollisionEnabled (Variables|Default|GetSphere) "QueryOnly")
  (Rendering|SetVisibility (Variables|Default|GetStaticMesh) true false))

(fn ConstructionScript)