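; BP_BonusZone is a one-shot trigger zone that starts a timed coin-collection challenge when an actor overlaps it.
; On overlap it caches the actor's CoinCollectorComponent, shows a HUD widget, spawns bonus coins at placed spawn points and disables its box collision.
; A looping timer counts down, removing the HUD and remaining coins on expiry.
; AddBonusCoin tallies pickups, crediting the collector only once every coin is collected.
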(event Custom|StartTimer
  (bind _result (Math|Float|DecrementFloat (Variables|Default|GetBonusTime))
    (:%20%20
      (bind _output_get (Variables|Default|SetBonusTime _result))
      (Default|UpdateTime (Variables|Default|GetWBP_HUDBonus) _output_get)
      (if (< (Variables|Default|GetBonusTime) 0.0)
        (CallFunction|ClearBonusZone)))))

(event Collision|EventActorBeginOverlap
  (params (OtherActor :type Actor%20Object%20Reference))
  (bind _spawnpoins (Variables|Default|GetSpawnPoins))
  (CallFunction|GetCoinCollector OtherActor)
  (bind _returnvalue (UserInterface|CreateWidget "/Game/HW3/Widget/WBP_HUDBonusZone.WBP_HUDBonusZone_C"))
  (bind _output_get (Variables|Default|SetWBP_HUDBonus _returnvalue))
  (UserInterface|Viewport|AddtoViewport _output_get 0)
  (Default|UpdateTime (Variables|Default|GetWBP_HUDBonus) (Variables|Default|GetBonusTime))
  (Variables|Default|SetSpawnedCoinsCount (Utilities|Array|Length _spawnpoins))
  (for _array_element _spawnpoins
    (bind _returnvalue_2 (Game|SpawnActorfromClass "/Game/HW3/Blueprints/BP_Coin.BP_Coin_C" (Math|Transform|MakeTransform (Transformation|GetActorLocation _array_element) "0, 0, 0" "1.000000,1.000000,1.000000") "Undefined" "MultiplyWithRoot" 0 0))
    (CallFunction|InitBonusCoin _returnvalue_2))
  (CallFunction|DisableZone)
  (bind _returnvalue_3 (Utilities|Time|SetTimerbyEvent (delegate Custom|StartTimer) 1.0 true))
  (Variables|Default|SetTimer _returnvalue_3))

(fn ConstructionScript)

(fn SetCoinCollector
  (Variables|Default|SetCoinCollector 0))

(fn AddBonusCoin
  (bind _result (Math|Integer|IncrementInt (Variables|Default|GetBonusCoins))
    (:%20%20
      (bind _output_get (Variables|Default|SetBonusCoins _result))
      (Default|UpdateBonusCoin (Variables|Default|GetWBP_HUDBonus) _output_get)
      (if (>= (Variables|Default|GetBonusCoins) (Variables|Default|GetSpawnedCoinsCount))
        (Default|AddCoins (Variables|Default|GetCoinCollector) (Variables|Default|GetBonusCoins))
        (Widget|RemovefromParent (Variables|Default|GetWBP_HUDBonus))
        (Utilities|Time|ClearandInvalidateTimerbyHandle (Variables|Default|GetTimer))))))

(fn DisableZone
  (Collision|SetCollisionEnabled (Variables|Default|GetBox) "NoCollision"))

(fn GetCoinCollector
  (params (TargetActor :type Actor%20Object%20Reference))
  (Variables|Default|SetCoinCollector (Actor|GetComponentbyClass TargetActor "/Game/HW3/Components/CoinCollectorComponent.CoinCollectorComponent_C")))

(fn DestroySpawnedCoinsAfterTimer
  (bind _spawnedcoins (Variables|Default|GetSpawnedCoins))
  (for _array_element _spawnedcoins
    (Utilities|IsValid _array_element
      (:Is%20Valid
        (Actor|DestroyActor _array_element))))
  (Utilities|Array|Clear _spawnedcoins))

(fn InitBonusCoin
  (params (InputPin :type BP%20Coin%20Object%20Reference))
  (Variables|/Game/HW3/Blueprints/BP_Coin.BP_Coin_C|SetIsBonusCoin InputPin true)
  (Variables|/Game/HW3/Blueprints/BP_Coin.BP_Coin_C|SetOwnerBonusZone InputPin self)
  (Utilities|Array|Add (Variables|Default|GetSpawnedCoins) InputPin))

(fn ClearBonusZone
  (Widget|RemovefromParent (Variables|Default|GetWBP_HUDBonus))
  (Utilities|Time|ClearandInvalidateTimerbyHandle (Variables|Default|GetTimer))
  (CallFunction|DestroySpawnedCoinsAfterTimer))