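; BP_Chest is a treasure chest that opens when the player touches it and hands out coins once.
; Overlapping the lid box plays a timeline that rotates the Scene component to swing the lid open.
; Overlapping the treasure box while open adds coins through the player's CoinCollectorComponent and hides the treasure.
; A Reset event restores the treasure and state flags, then animates the lid closed with a second timeline.
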(event OnComponentBeginOverlap(BoxLid)
  (params (OverlappedComponent :type Primitive%20Component%20Object%20Reference) (OtherActor :type Actor%20Object%20Reference) (OtherComp :type Primitive%20Component%20Object%20Reference) (OtherBodyIndex :type Integer) (bFromSweep :type Boolean) (SweepResult :type Hit%20Result%20Structure%20%28by%20ref%29))
  (if (and (== OtherActor (Game|GetPlayerCharacter 0)) (not (Variables|Default|GetIsOpen)))
    (Variables|Default|SetIsOpen true)
    (bind _opening (Timeline|OpeningLid PlayFromStart)
      (:Update
        (Transformation|SetRelativeRotation (Variables|Default|GetScene) (Math|Rotator|Lerp(Rotator) "0, 0, 0" "0.000000,0.000000,-90.000000" _opening) false false)))))

(event OnComponentBeginOverlap(BoxTreasure)
  (params (OverlappedComponent :type Primitive%20Component%20Object%20Reference) (OtherActor :type Actor%20Object%20Reference) (OtherComp :type Primitive%20Component%20Object%20Reference) (OtherBodyIndex :type Integer) (bFromSweep :type Boolean) (SweepResult :type Hit%20Result%20Structure%20%28by%20ref%29))
  (if (Math|Boolean|ANDBoolean (== OtherActor (Game|GetPlayerCharacter 0)) (Variables|Default|GetIsOpen) (not (Variables|Default|GetWasStolen)))
    (Default|AddCoins (Actor|GetComponentbyClass OtherActor "/Game/HW3/Components/CoinCollectorComponent.CoinCollectorComponent_C") (Variables|Default|GetNumberOfCoins))
    (Variables|Default|SetWasStolen true)
    (Rendering|SetVisibility (Variables|Default|GetTreasure) false false)))

(event EventReset
  (Variables|Default|SetWasStolen false)
  (Rendering|SetVisibility (Variables|Default|GetTreasure) true false)
  (Variables|Default|SetIsOpen false)
  (bind _opening (Timeline|Timeline PlayFromStart)
    (:Update
      (Transformation|SetRelativeRotation (Variables|Default|GetScene) (Math|Rotator|Lerp(Rotator) "0.000000,0.000000,-90.000000" "0, 0, 0" _opening) false false))))

(fn ConstructionScript)