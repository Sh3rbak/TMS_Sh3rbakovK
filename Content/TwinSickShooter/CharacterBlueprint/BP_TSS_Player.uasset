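; Player character for a top-down twin-stick shooter, moved by axis input and aimed with the mouse cursor.
; Each tick it traces under the cursor and smoothly interpolates toward the hit point, flattening the look-at to the hit's height so it only yaws.
; Movement follows control yaw, independent of facing.
; BeginPlay caches the controller, shows the cursor and sets the combat component's starting weapon; FindPlayer returns self.
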(event Custom|Move
  (params (x :type Float%20%28single-precision%29) (y :type Float%20%28single-precision%29))
  (CallFunction|MoveXY x y))

(event EventBeginPlay
  (bind _returnvalue (Game|GetPlayerController 0))
  (Variables|Default|SetPlayerController _returnvalue)
  (Variables|/Script/Engine.PlayerController|SetbShowMouseCursor _returnvalue true)
  (Variables|/Game/TwinSickShooter/Components/CombatComponent.CombatComponent_C|SetCurrectWeapon (Variables|Default|GetCombatComp) "NewEnumerator1"))

(event EventTick
  (params (DeltaSeconds :type Float%20%28single-precision%29))
  (CallFunction|RotateCharinDirectionOfCursor))

(fn ConstructionScript)

(fn RotateCharinDirectionOfCursor
  (bind _playercontroller (Variables|Default|GetPlayerController))
  (bind (_hitresult _returnvalue) (Game|Player|GetHitResultUnderCursorbyChannel _playercontroller "TraceTypeQuery1" true))
  (if _returnvalue
    (Variables|Default|SetCacheLocation (.Location (Collision|BreakHitResult _hitresult)))
    (Transformation|SetActorRotation (CallFunction|GetChangingRotation))))

(fn GetChangingRotation
  (bind _returnvalue (Transformation|GetActorLocation))
  (bind _cachelocation (Variables|Default|GetCacheLocation))
  (bind (_x _y _z) (Math|Vector|BreakVector _cachelocation))
  (return (Math|Interpolation|RInterpTo (Transformation|GetActorRotation) (Math|Rotator|FindLookatRotation (Math|Vector|MakeVector (.x _returnvalue) (.y _returnvalue) _z) (Math|Vector|MakeVector _x _y _z)) (Utilities|Time|GetWorldDeltaSeconds) 0.0)))

(fn MoveXY
  (params (InputPin :type Float%20%28single-precision%29) (ScaleValue :type Float%20%28single-precision%29))
  (bind _returnvalue (Pawn|GetControlRotation :!class /Script/Engine.Pawn))
  (Pawn|Input|AddMovementInput (Math|Vector|GetRightVector (Math|Rotator|MakeRotator 0.0 0.0 (.yaw _returnvalue))) InputPin false)
  (Pawn|Input|AddMovementInput (Math|Vector|GetForwardVector (Math|Rotator|MakeRotator 0.0 0.0 (.yaw _returnvalue))) ScaleValue false))

(fn FindPlayer
  (return self))