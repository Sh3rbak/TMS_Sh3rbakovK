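; Interactable swing door for the twin-stick shooter, toggled open and closed on interact and closed when anything stops overlapping its sphere.
; A timeline lerps between the rotation saved at BeginPlay and a fixed ±90° target, reversing to close.
; GetDirectionOpening picks the sign from player 0's position unless already moving.
; Its comments describe a 2D cross product, but the math subtracts components where it should multiply.
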(event OnComponentEndOverlap(Sphere)
  (params (OverlappedComponent :type Primitive%20Component%20Object%20Reference) (OtherActor :type Actor%20Object%20Reference) (OtherComp :type Primitive%20Component%20Object%20Reference) (OtherBodyIndex :type Integer))
  (Variables|Default|SetIsCloused false)
  (CallFunction|PushDoor))

(event Custom|PushDoor
  (if (Variables|Default|GetIsCloused)
    (Variables|Default|SetIsCloused false)
    (if (Variables|Default|GetIsMoving)
      (bind _alpha (Timeline|Timeline Play)
        (:Update
          (Transformation|SetRelativeRotation (Variables|Default|GetScene) (Math|Rotator|Lerp(Rotator) (Variables|Default|GetClousedRotation) (Variables|Default|GetOpenRotation) _alpha) false false)
          (Variables|Default|SetIsMoving true))
        (:Finished
          (Variables|Default|SetIsMoving false)))
      (else
        (Variables|Default|SetOpenRotation (CallFunction|GetDirectionOpening))
        (Timeline|Timeline Play)))
    (else
      (Variables|Default|SetIsCloused true)
      (Timeline|Timeline Reverse))))

(event EventBeginPlay
  (|CallParentFunction)
  (Variables|Default|SetClousedRotation (Variables|/Script/Engine.SceneComponent|GetRelativeRotation (Variables|Default|GetScene))))

(event Collision|EventActorBeginOverlap
  (params (OtherActor :type Actor%20Object%20Reference))
  (|CallParentFunction OtherActor) ; This node is disabled and will not be called.\nDrag off pins to build functionality.
)

(event EventTick
  (params (DeltaSeconds :type Float%20%28single-precision%29))
  (|CallParentFunction DeltaSeconds) ; This node is disabled and will not be called.\nDrag off pins to build functionality.
)

(event EventInteractChar
  (params (Character :type Actor%20Object%20Reference))
  (CallFunction|PushDoor))

(fn ConstructionScript
  (|CallParentFunction))

(fn GetDirectionOpening
  (bind _returnvalue (Game|GetPlayerCharacter 0))
  (bind _returnvalue_2 (Transformation|GetActorLocation))
  (bind _scene (Variables|Default|GetScene))
  (bind _returnvalue_3 (Transformation|GetActorLocation _returnvalue))
  (bind _returnvalue_4 (Math|Vector|GetForwardVector _scene))
  (bind _returnvalue_5 (- _returnvalue_3 _returnvalue_2))
  (return (Math|Rotator|SelectRotator "0.000000,90.000000,0.000000" "0.000000,-90.000000,0.000000" (> (- (- (.x _returnvalue_4) (.y _returnvalue_5)) (- (.y _returnvalue_4) (.x _returnvalue_5))) 0.0))))