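; Twin-stick shooter enemy that turns toward a target pawn and advances along its own forward vector.
; On BeginPlay it targets the first Pawn found in the level, without checking that it is the player.
; Each tick it smoothly interpolates its rotation toward that target and moves forward with a swept offset.
; Health component change events update the percentage on its widget health bar.
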(event Custom|OnHealthChange_Event
  (CallFunction|UpdateHealthBar))

(event EventBeginPlay
  (CallFunction|TargetPawnPlayer)
  (EventDispatchers|AssignOnHealthChange (Variables|Default|GetHealthComponentTSS) (delegate Custom|OnHealthChange_Event)))

(event EventTick
  (params (DeltaSeconds :type Float%20%28single-precision%29))
  (CallFunction|InterpolationRotation)
  (CallFunction|MovetoTarget))

(fn ConstructionScript)

(fn TargetPawnPlayer
  (bind _outactors (Actor|GetAllActorsOfClass "/Script/Engine.Pawn"))
  (if (Utilities|Array|IsValidIndex _outactors)
    (Variables|Default|SetTargetPawn (Utilities|Array|Get(acopy) _outactors))))

(fn InterpolationRotation
  (Variables|Default|GetTargetPawn
    (:then
      (Transformation|SetActorRotation (Math|Interpolation|RInterpTo (Transformation|GetActorRotation) (Math|Rotator|FindLookatRotation (Transformation|GetActorLocation) (Transformation|GetActorLocation (Variables|Default|GetTargetPawn))) (Utilities|Time|GetWorldDeltaSeconds) (Variables|Default|GetInterp%20Speed))))
    (:else)))

(fn MovetoTarget
  (Transformation|AddActorWorldOffset (* (Transformation|GetActorForwardVector) (* (Utilities|Time|GetWorldDeltaSeconds) (Variables|Default|GetSpeedMove))) true))

(fn UpdateHealthBar
  (bind _aswbp_tss_health_bar (Utilities|Casting|CastToWBP_TSS_HealthBar (UserInterface|GetWidget (Variables|Default|GetWidget))))
  (Progress|SetPercent (Variables|/Game/TwinSickShooter/Widget/WBP_TSS_HealthBar.WBP_TSS_HealthBar_C|GetHealthBar _aswbp_tss_health_bar) (Variables|/Game/TwinSickShooter/Component/HealthComponentTSS.HealthComponentTSS_C|GetHealthPercent (Variables|Default|GetHealthComponentTSS))))