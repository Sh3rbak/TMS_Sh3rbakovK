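; BP_TSS_Heal is a heart health pickup for the TwinSickShooter game.
; When an actor overlaps its sphere, it finds that actor's HealthComponentTSS and heals it by HealAmount if health is below maximum.
; HideActor and ShowActor toggle the heart's visibility and the sphere's query collision, but the overlap event calls neither, so healing alone does not consume the pickup.
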(event OnComponentBeginOverlap(Sphere)
  (params (OverlappedComponent :type Primitive%20Component%20Object%20Reference) (OtherActor :type Actor%20Object%20Reference) (OtherComp :type Primitive%20Component%20Object%20Reference) (OtherBodyIndex :type Integer) (bFromSweep :type Boolean) (SweepResult :type Hit%20Result%20Structure%20%28by%20ref%29))
  (bind _returnvalue (Actor|GetComponentbyClass OtherActor "/Game/TwinSickShooter/Blueprints/Component/HealthComponentTSS.HealthComponentTSS_C"))
  (Utilities|IsValid _returnvalue
    (:Is%20Valid
      (bind _output_get (Variables|Default|SetHealthComp _returnvalue))
      (if (< (Variables|/Game/TwinSickShooter/Blueprints/Component/HealthComponentTSS.HealthComponentTSS_C|GetCurrectHealth _output_get) (Variables|/Game/TwinSickShooter/Blueprints/Component/HealthComponentTSS.HealthComponentTSS_C|GetMaxHealth _output_get))
        (Default|Heal _output_get (Variables|Default|GetHeal%20Amount))))))

(fn ConstructionScript)

(fn HideActor
  (Collision|SetCollisionEnabled (Variables|Default|GetSphere) "NoCollision")
  (Rendering|SetVisibility (Variables|Default|GetHeart) false false))

(fn ShowActor
  (Rendering|SetVisibility (Variables|Default|GetHeart) true false)
  (Collision|SetCollisionEnabled (Variables|Default|GetSphere) "QueryOnly"))