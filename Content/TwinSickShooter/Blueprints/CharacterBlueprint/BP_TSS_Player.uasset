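; Player character for a top-down shooter that moves with Enhanced Input, turns toward the mouse cursor, and fights with a pistol.
; Weapon switching swaps the hand mesh and animation blueprint.
; Firing consumes AmmoComponentTSS rounds, then line-traces from the muzzle to damage HealthComponentTSS, with effects and misfire audio.
; Holding scope aims the trace at the exact cursor point instead of horizontally; ammo changes update a HUD widget.
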(event Input|EnhancedActionEvents|EnhancedInputActionIA_TSS_Scope
  (params (ActionValue :type Boolean) (ElapsedSeconds :type Float%20%28double-precision%29) (TriggeredSeconds :type Float%20%28double-precision%29) (InputAction :type Input%20Action%20Object%20Reference :default "/Game/TwinSickShooter/Input/IA_TSS_Scope.IA_TSS_Scope"))
  (:Started
    (Variables|Default|SetTypeAim "NewEnumerator1"))
  (:Completed
    (Variables|Default|SetTypeAim "NewEnumerator0")))

(event Input|EnhancedActionEvents|EnhancedInputActionIA_TSS_Move
  (params (ActionValue :type Vector%202D%20Structure) (ElapsedSeconds :type Float%20%28double-precision%29) (TriggeredSeconds :type Float%20%28double-precision%29) (InputAction :type Input%20Action%20Object%20Reference :default "/Game/TwinSickShooter/Input/IA_TSS_Move.IA_TSS_Move"))
  (bind (_x _y) (Math|Vector2D|BreakVector2D ActionValue))
  (CallFunction|MoveXY _x _y))

(event Input|EnhancedActionEvents|EnhancedInputActionIA_TSS_Jump
  (params (ActionValue :type Boolean) (ElapsedSeconds :type Float%20%28double-precision%29) (TriggeredSeconds :type Float%20%28double-precision%29) (InputAction :type Input%20Action%20Object%20Reference :default "/Game/TwinSickShooter/Input/IA_TSS_Jump.IA_TSS_Jump"))
  (:Started
    (Character|Jump))
  (:Completed
    (Character|StopJumping)))

(event Input|EnhancedActionEvents|EnhancedInputActionIA_TSS_Fire
  (params (ActionValue :type Boolean) (ElapsedSeconds :type Float%20%28double-precision%29) (TriggeredSeconds :type Float%20%28double-precision%29) (InputAction :type Input%20Action%20Object%20Reference :default "/Game/TwinSickShooter/Input/IA_TSS_Fire.IA_TSS_Fire"))
  (:Started
    (if (CallFunction|CheckPossibilityShot)
      (switch Utilities|FlowControl|Switch|SwitchonEnum_TSS_Weapons (Variables|Default|GetCurrectWeapon)
        (:NewEnumerator1
          (Audio|PlaySoundatLocation "/Game/TwinSickShooter/Sound/SW_TSS_Shot.SW_TSS_Shot" (Transformation|GetActorLocation) "0, 0, 0" 1.0 1.0 0.0 0 0 0 0)
          (CallFunction|SpawnMuzzleEffect)
          (bind _hitactor (CallFunction|SpawnLineTraceUntilShot))
          (Utilities|IsValid _hitactor
            (:Is%20Valid
              (Utilities|IsValid (Actor|GetComponentbyClass _hitactor "/Game/TwinSickShooter/Blueprints/Component/HealthComponentTSS.HealthComponentTSS_C")
                (:Is%20Valid
                  (Default|TakeDamage (Actor|GetComponentbyClass _hitactor "/Game/TwinSickShooter/Blueprints/Component/HealthComponentTSS.HealthComponentTSS_C") 1e+01)))))))
      (else
        (CallFunction|PlayMisfire)))))

(event Input|EnhancedActionEvents|EnhancedInputActionIA_TSS_Reload
  (params (ActionValue :type Boolean) (ElapsedSeconds :type Float%20%28double-precision%29) (TriggeredSeconds :type Float%20%28double-precision%29) (InputAction :type Input%20Action%20Object%20Reference :default "/Game/TwinSickShooter/Input/IA_TSS_Reload.IA_TSS_Reload"))
  (:Started
    (switch Utilities|FlowControl|Switch|SwitchonEnum_TSS_Weapons (Variables|Default|GetCurrectWeapon)
      (:NewEnumerator1
        (Default|Reload (Variables|Default|GetAmmoComponentTSS))
        (CallFunction|UpdateWBPAmmo)))))

(event EventBeginPlay
  (bind _returnvalue (Game|GetPlayerController 0))
  (Variables|Default|SetPlayerController _returnvalue)
  (Variables|/Script/Engine.PlayerController|SetbShowMouseCursor _returnvalue true)
  (CallFunction|ChangeWeapon "NewEnumerator0")
  (CallFunction|SetWBPAmmo))

(event EventTick
  (params (DeltaSeconds :type Float%20%28single-precision%29))
  (CallFunction|RotateCharinDirectionOfCursor))

(event EventChangeWeapon
  (params (NewParam :type Enum_TSS_Weapons%20Enum :default "NewEnumerator0"))
  (bind _output_get (Variables|Default|SetCurrectWeapon NewParam))
  (switch Utilities|FlowControl|Switch|SwitchonEnum_TSS_Weapons _output_get
    (:NewEnumerator0
      (Components|SkeletalMesh|SetAnimInstanceClass (Variables|Character|GetMesh) "/Game/Characters/Mannequins/Anims/Unarmed/ABP_Unarmed.ABP_Unarmed_C")
      (Components|StaticMesh|SetStaticMesh (Variables|Default|GetHandGun) 0))
    (:NewEnumerator1
      (Animation|PlayAnimMontage "/Game/Characters/Mannequins/Anims/Pistol/MM_Pistol_Equip_Montage.MM_Pistol_Equip_Montage" 1.0 "None")
      (Components|StaticMesh|SetStaticMesh (Variables|Default|GetHandGun) "/Game/TwinSickShooter/Mesh/Pistol/SM_Pistol.SM_Pistol")
      ;[0.15 0.15 0.15 0.5] Чтобы анимация была не столь кривой
      (Utilities|FlowControl|Delay 0.8)
      (Components|SkeletalMesh|SetAnimInstanceClass (Variables|Character|GetMesh) "/Game/Characters/Mannequins/Anims/Pistol/ABP_HandWeapon.ABP_HandWeapon_C"))))

(fn ConstructionScript)

(fn RotateCharinDirectionOfCursor
  (bind _playercontroller (Variables|Default|GetPlayerController))
  (bind (_hitresult _returnvalue) (Game|Player|GetHitResultUnderCursorbyChannel _playercontroller "TraceTypeQuery2" true))
  (if _returnvalue
    (Variables|Default|SetCacheLocation (.Location (Collision|BreakHitResult _hitresult)))
    (Transformation|SetActorRotation (CallFunction|GetChangingRotation))))

(fn GetChangingRotation
  (bind _returnvalue (Transformation|GetActorLocation))
  (bind _cachelocation (Variables|Default|GetCacheLocation))
  (bind (_x _y _z) (Math|Vector|BreakVector _cachelocation))
  (return (Math|Interpolation|RInterpTo (Transformation|GetActorRotation) (Math|Rotator|FindLookatRotation (Math|Vector|MakeVector (.x _returnvalue) (.y _returnvalue) _z) (Math|Vector|MakeVector _x _y _z)) (Utilities|Time|GetWorldDeltaSeconds) 0.0)))

(fn MoveXY
  (params (InputPin :type Float%20%28single-precision%29) (ScaleValue :type Float%20%28single-precision%29))
  (bind _returnvalue (Pawn|GetControlRotation :!class /Script/Engine.Pawn))
  (Pawn|Input|AddMovementInput (Math|Vector|GetRightVector (Math|Rotator|MakeRotator 0.0 0.0 (.yaw _returnvalue))) InputPin false)
  (Pawn|Input|AddMovementInput (Math|Vector|GetForwardVector (Math|Rotator|MakeRotator 0.0 0.0 (.yaw _returnvalue))) ScaleValue false))

(fn SpawnMuzzleEffect
  (bind _bulletsocket (Variables|Default|GetBulletSocket))
  (bind _returnvalue (Transformation|GetWorldRotation _bulletsocket))
  ;[0.15 0.15 0.15 0.5] Effect vfx in direction shot
  (Niagara|SpawnSystematLocation "/Game/MuzzleFlash/MuzzleFlash/Niagara/NS_MuzzleFlash.NS_MuzzleFlash" (Transformation|GetWorldLocation _bulletsocket) (Math|Rotator|MakeRotator (.roll _returnvalue) (.pitch _returnvalue) (- (.yaw _returnvalue) 9e+01))))

(fn SpawnLineTraceUntilShot
  (bind (_outhit _returnvalue) (Collision|LineTraceByChannel (Transformation|GetWorldLocation (Variables|Default|GetBulletSocket)) (CallFunction|GetEndOfLine) "TraceTypeQuery2" false 0 "ForDuration" true "(R=1.000000,G=0.000000,B=0.000000,A=1.000000)" "(R=0.000000,G=1.000000,B=0.000000,A=1.000000)" 1.0))
  (if _returnvalue
    (Niagara|SpawnSystematLocation "/Game/MuzzleFlash/MuzzleFlash/Niagara/NS_MuzzleFlash.NS_MuzzleFlash" (.Location (Collision|BreakHitResult _outhit)) (Math|Rotator|MakeRotator 9e+01 0.0 0.0))
    (return (.HitActor (Collision|BreakHitResult _outhit)))))

(fn GetEndOfLine
  (bind _output_get (LocalVariables|SetStartTrace (Transformation|GetWorldLocation (Variables|Default|GetBulletSocket))))
  (bind _output_get_2 (LocalVariables|SetDeltaVector (- (Variables|Default|GetCacheLocation) _output_get)))
  (return (+ (LocalVariables|GetStartTrace) (* (Utilities|Select :Index (Variables|Default|GetTypeAim) :NewEnumerator0 (Class|KismetMathLibrary|VectorNormal2D _output_get_2 0.0001) :NewEnumerator1 (Math|Vector|Normalize _output_get_2)) (Variables|Default|GetTraceRange)))))

(fn UpdateWBPAmmo
  (bind _ammocomponenttss (Variables|Default|GetAmmoComponentTSS))
  (Default|CallOnChangeAmmo (Variables|Default|GetWBP_Ammo) (Variables|/Game/TwinSickShooter/Blueprints/Component/AmmoComponentTSS.AmmoComponentTSS_C|GetCurrectAmmo _ammocomponenttss) (Variables|/Game/TwinSickShooter/Blueprints/Component/AmmoComponentTSS.AmmoComponentTSS_C|GetCurrectNumMagazins _ammocomponenttss)))

(fn CheckPossibilityShot
  (if (Utilities|Enum|NotEqual(Enum) (Variables|Default|GetCurrectWeapon) "NewEnumerator0")
    (bind _wasshot (Default|Shot (Variables|Default|GetAmmoComponentTSS)))
    (CallFunction|UpdateWBPAmmo)
    (return _wasshot)
    (else
      (return true))))

(fn PlayMisfire
  (if (not (Variables|/Game/TwinSickShooter/Blueprints/Component/AmmoComponentTSS.AmmoComponentTSS_C|GetIsReloading (Variables|Default|GetAmmoComponentTSS)))
    (Audio|PlaySoundatLocation "/Game/TwinSickShooter/Sound/SW_TSS_Misfire.SW_TSS_Misfire" (Transformation|GetActorLocation) "0, 0, 0" 1.0 1.0 0.0 0 0 0 0)))

(fn SetWBPAmmo
  (bind _returnvalue (UserInterface|CreateWidget "/Game/TwinSickShooter/Widget/WBP_Ammo.WBP_Ammo_C"))
  (bind _output_get (Variables|Default|SetWBP_Ammo _returnvalue))
  (UserInterface|Viewport|AddtoViewport _output_get 0))

(fn PickupAmmo
  (bind _success (Default|PickupAmmo (Variables|Default|GetAmmoComponentTSS)))
  (if _success
    (CallFunction|UpdateWBPAmmo)
    (return _success)
    (else
      (return _success))))

(fn WeaponinHands
  (return (Variables|Default|GetCurrectWeapon)))