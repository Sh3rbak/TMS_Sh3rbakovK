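; Ammo component for the twin-stick shooter that tracks the loaded magazine and spare magazine count.
; Shot spends a round outside reloads, broadcasts the change and returns whether another shot remains possible.
; Reload swaps in a spare magazine immediately, then blocks firing until the owning Character's pistol montage completes.
; PickupAmmo adds a spare up to the limit, or refills an empty magazine directly, and reports success.
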(event Custom|Reload
  (if (and (< (Variables|Default|GetCurrectAmmo) (Variables|Default|GetMaxSizeMagazin)) (> (Variables|Default|GetCurrectNumMagazins) 0))
    (Variables|Default|SetCurrectAmmo (Variables|Default|GetMaxSizeMagazin))
    (Math|Integer|DecrementInt (Variables|Default|GetCurrectNumMagazins)
      (:%20%20
        (Variables|Default|SetIsReloading true)
        ;[0.15 0.15 0.15 0.5] Каст на базовые классы не загружает большой объем данных, т.к. в них нет тяжелых данных
        (bind _ascharacter (Utilities|Casting|CastToCharacter (Components|GetOwner)))
        (Animation|Montage|PlayMontage (Variables|/Script/Engine.Character|GetMesh _ascharacter) "/Game/Characters/Mannequins/Anims/Pistol/MM_Pistol_Reload_Montage.MM_Pistol_Reload_Montage"
          (:OnCompleted
            (Variables|Default|SetIsReloading false)))))))

(fn Shot
  (bind _isreloading (Variables|Default|GetIsReloading))
  (bind _currectammo (Variables|Default|GetCurrectAmmo))
  (bind _returnvalue (not _isreloading))
  (bind _returnvalue_2 (> _currectammo 0))
  (bind _returnvalue_3 (and _returnvalue_2 _returnvalue))
  (if _returnvalue_3
    (Math|Integer|DecrementInt (Variables|Default|GetCurrectAmmo)
      (:%20%20
        (Default|CallOnChangeAmmoinMagazine)
        (return _returnvalue_3)))
    (else
      (return _returnvalue_3))))

(fn PickupAmmo
  (bind _currectnummagazins (Variables|Default|GetCurrectNumMagazins))
  (bind _maxnummagazins (Variables|Default|GetMaxNumMagazins))
  (bind _returnvalue (< _currectnummagazins _maxnummagazins))
  (if (> (Variables|Default|GetCurrectAmmo) 0)
    (if _returnvalue
      (Math|Integer|IncrementInt (Variables|Default|GetCurrectNumMagazins)
        (:%20%20
          (return true)))
      (else
        (return _returnvalue)))
    (else
      (Variables|Default|SetCurrectAmmo (Variables|Default|GetMaxSizeMagazin))
      (return true))))