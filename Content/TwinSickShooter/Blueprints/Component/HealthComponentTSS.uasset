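; Health component for the TwinSickShooter game that tracks an owner's current and maximum health, starting full on BeginPlay.
; TakeDamage and Heal ignore non-positive amounts and dead owners, clamp health between zero and max, then fire OnHealthChange with the value and percentage.
; Reaching zero health sets IsDead and fires OnDeath once, while Heal also skips when already full.
; Both paths print the health percentage as debug output.
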(event EventBeginPlay
  (Variables|Default|SetCurrectHealth (Variables|Default|GetMaxHealth)))

(event EventTick
  (params (DeltaSeconds :type Float%20%28single-precision%29)))

(fn TakeDamage
  (params (Damage%20Amount :type Float%20%28double-precision%29))
  (bind _percent (CallFunction|GetHealthPercent))
  (Variables|Default|SetDamageAmount Damage%20Amount)
  (if (or (Variables|Default|GetIsDead) (<= (Variables|Default|GetDamageAmount) 0.0))
    (return)
    (else
      (bind _currhp (CallFunction|UpdateCurrectHealthAfterDamage))
      (Default|CallOnHealthChange _currhp _percent)
      (Development|PrintString (Utilities|String|ToString(Float) _percent))
      (if (== (Variables|Default|GetCurrectHealth) 0.0)
        (Variables|Default|SetIsDead true)
        (Default|CallOnDeath)
        (return)))))

(fn UpdateCurrectHealthAfterDamage
  (bind _output_get (Variables|Default|SetCurrectHealth (Math|Float|Clamp(Float) (- (Variables|Default|GetCurrectHealth) (Variables|Default|GetDamageAmount)) 0.0 (Variables|Default|GetMaxHealth))))
  (return _output_get))

(fn Heal
  (params (HealAmount :type Float%20%28double-precision%29))
  (bind _percent (CallFunction|GetHealthPercent))
  (Variables|Default|SetHeal%20Amount HealAmount)
  (if (Math|Boolean|ORBoolean (Variables|Default|GetIsDead) (>= (Variables|Default|GetCurrectHealth) (Variables|Default|GetMaxHealth)) (<= (Variables|Default|GetHeal%20Amount) 0.0))
    (return)
    (else
      (bind _curhp (CallFunction|UpdateCurrectHealthAfterHeal))
      (Default|CallOnHealthChange _curhp _percent)
      (Development|PrintString (Utilities|String|ToString(Float) _percent)))))

(fn UpdateCurrectHealthAfterHeal
  (bind _output_get (Variables|Default|SetCurrectHealth (Math|Float|Clamp(Float) (+ (Variables|Default|GetCurrectHealth) (Variables|Default|GetHeal%20Amount)) 0.0 (Variables|Default|GetMaxHealth))))
  (return _output_get))

(fn GetHealthPercent
  (return (/ (Variables|Default|GetCurrectHealth) (Variables|Default|GetMaxHealth))))