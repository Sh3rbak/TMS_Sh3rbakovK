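; Base interactable actor for the TwinSickShooter game that tells the player when it is in range and shows a prompt widget.
; A Sphere overlap checks for player character 0 and passes entering or leaving to its InteractComponentTSS through InteractOverlap.
; Hovered and UnHovered events show or hide the Widget component.
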(event OnComponentBeginOverlap(Sphere)
  (params (OverlappedComponent :type Primitive%20Component%20Object%20Reference) (OtherActor :type Actor%20Object%20Reference) (OtherComp :type Primitive%20Component%20Object%20Reference) (OtherBodyIndex :type Integer) (bFromSweep :type Boolean) (SweepResult :type Hit%20Result%20Structure%20%28by%20ref%29))
  (bind _returnvalue (Actor|GetComponentbyClass OtherActor "/Game/TwinSickShooter/Blueprints/InteractObject/InteractComponentTSS.InteractComponentTSS_C"))
  (if (CallFunction|IsPlayerChar OtherActor)
    (Utilities|IsValid _returnvalue
      (:Is%20Valid
        (Default|InteractOverlap _returnvalue true)))))

(event OnComponentEndOverlap(Sphere)
  (params (OverlappedComponent :type Primitive%20Component%20Object%20Reference) (OtherActor :type Actor%20Object%20Reference) (OtherComp :type Primitive%20Component%20Object%20Reference) (OtherBodyIndex :type Integer))
  (bind _returnvalue (Actor|GetComponentbyClass OtherActor "/Game/TwinSickShooter/Blueprints/InteractObject/InteractComponentTSS.InteractComponentTSS_C"))
  (if (CallFunction|IsPlayerChar OtherActor)
    (Utilities|IsValid _returnvalue
      (:Is%20Valid
        (Default|InteractOverlap _returnvalue false)))))

(event EventBeginPlay)

(event Collision|EventActorBeginOverlap
  (params (OtherActor :type Actor%20Object%20Reference)))

(event EventTick
  (params (DeltaSeconds :type Float%20%28single-precision%29)))

(event EventUnHovered
  (Rendering|SetVisibility (Variables|Default|GetWidget) false false))

(event EventHovered
  (Rendering|SetVisibility (Variables|Default|GetWidget) true false))

(fn ConstructionScript)

(fn IsPlayerChar
  (params (OtherActor :type Object%20Object%20Reference))
  (return (== OtherActor (Game|GetPlayerCharacter 0))))