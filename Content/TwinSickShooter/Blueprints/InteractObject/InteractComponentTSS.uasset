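; Player interaction component for TwinSickShooter that finds, highlights and triggers interactable objects.
; Overlap events are counted, and a looping timer runs detection only while the count is above zero.
; Each tick sphere-traces from the screen-center deprojection to the owner, sending hover and unhover messages as the hit "InteractObj"-tagged actor changes.
; The Interact input passes the owner to the current target, and clearing happens when the count returns to zero.
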(event Custom|InteractOverlap
  (params (IsOverlap :type Boolean))
  (Utilities|FlowControl|Sequence
    (:then_0
      (CallFunction|CountOverlapObject IsOverlap))
    (:then_1
      (CallFunction|UpdateStateDebugState IsOverlap))))

(event Custom|DrawDebugTrace
  (bind _returnvalue (Utilities|Time|SetTimerbyFunctionName 0 "DetectedTirgetSight" 0.1 true))
  (Variables|Default|SetTimer _returnvalue))

(event Input|EnhancedActionEvents|EnhancedInputActionIA_TSS_Interact
  (params (ActionValue :type Boolean) (ElapsedSeconds :type Float%20%28double-precision%29) (TriggeredSeconds :type Float%20%28double-precision%29) (InputAction :type Input%20Action%20Object%20Reference :default "/Game/TwinSickShooter/Input/IA_TSS_Interact.IA_TSS_Interact"))
  (:Started
    (if (Utilities|IsValid (Variables|Default|GetCurrentInteract))
      (Class|BPITSSInteractable|InteractChar(Message) (Variables|Default|GetCurrentInteract) (Components|GetOwner)))))

(fn DetectedTirgetSight
  (bind (_outhit _returnvalue) (Collision|SphereTraceByChannel (.StartTrace (CallFunction|CalculateTrace (Game|GetPlayerController 0))) (Transformation|GetActorLocation (Components|GetOwner)) 1.5e+02 "TraceTypeQuery3" false 0 "ForDuration" true "(R=1.000000,G=0.000000,B=0.000000,A=1.000000)" "(R=0.000000,G=1.000000,B=0.000000,A=1.000000)" 0.2))
  (if _returnvalue
    (if (Actor|ActorHasTag (.HitActor (Collision|BreakHitResult _outhit)) "InteractObj")
      (CallFunction|SetCurrentInteract (.HitActor (Collision|BreakHitResult _outhit)))
      (else
        (CallFunction|ClearCurrectInteractable)))
    (else
      (CallFunction|ClearCurrectInteractable))))

(fn CalculateTrace
  (params (Controller :type Player%20Controller%20Object%20Reference))
  (bind (_sizex _sizey) (HUD|GetViewportSize Controller))
  (bind _returnvalue (/ _sizex 2))
  (bind _returnvalue_2 (/ _sizey 2))
  (bind _returnvalue_3 (Math|Conversions|ToFloat(Integer) _returnvalue))
  (bind _returnvalue_4 (Math|Conversions|ToFloat(Integer) _returnvalue_2))
  (bind (_worldlocation _worlddirection) (Class|PlayerController|DeprojectScreenPositiontoWorld Controller _returnvalue_3 _returnvalue_4))
  (return _worldlocation (+ _worldlocation (* _worlddirection 1.5e+03))))

(fn SetCurrentInteract
  (params (NewInteract :type Actor%20Object%20Reference))
  ;[0.15 0.15 0.15 0.5] Проверка изменения объекта в зоне взаимодействия.
  (if (not (== NewInteract (Variables|Default|GetCurrentInteract)))
    (CallFunction|ClearCurrectInteractable)
    (bind _output_get (Variables|Default|SetCurrentInteract NewInteract))
    (Utilities|IsValid _output_get
      (:Is%20Valid
        (Class|BPITSSInteractable|Hovered(Message) NewInteract))
      (:Is%20Not%20Valid
        (Variables|Default|SetCurrentInteract 0)))))

(fn ClearCurrectInteractable
  (Utilities|FlowControl|Sequence
    (:then_0
      (Utilities|IsValid (Variables|Default|GetCurrentInteract)
        (:Is%20Valid
          (Class|BPITSSInteractable|UnHovered(Message) (Variables|Default|GetCurrentInteract)))))
    (:then_1
      (Variables|Default|SetCurrentInteract 0))))

(fn CountOverlapObject
  (params (IsOverlap :type Boolean))
  (Variables|Default|SetOverlapCount (Math|Integer|Max(Integer) (+ (Variables|Default|GetOverlapCount) (select IsOverlap 1 -1)))))

(fn UpdateStateDebugState
  (params (Condition :type Boolean))
  (if Condition
    (if (== (Variables|Default|GetOverlapCount) 1)
      (CallFunction|DrawDebugTrace))
    (elif (== (Variables|Default|GetOverlapCount) 0)
      (Utilities|Time|ClearandInvalidateTimerbyHandle (Variables|Default|GetTimer))
      (CallFunction|ClearCurrectInteractable))))