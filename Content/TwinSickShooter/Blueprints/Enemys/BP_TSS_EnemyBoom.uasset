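; BP_TSS_EnemyBoom is a suicide-bomber enemy for the twin-stick shooter that detonates when close to the player.
; A looping timer started on BeginPlay checks its distance to the player character every half second.
; Within the detonation distance, it deals damage through the player's HealthComponentTSS and destroys itself.
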(event Custom|DetonateNearChar
  (if (<= (Math|Vector|Distance(Vector) (Transformation|GetActorLocation (Game|GetPlayerCharacter 0)) (Transformation|GetActorLocation)) (Variables|Default|GetDistanceToDetonate))
    (Default|TakeDamage (Actor|GetComponentbyClass (Game|GetPlayerCharacter 0) "/Game/TwinSickShooter/Blueprints/Component/HealthComponentTSS.HealthComponentTSS_C") (Variables|Default|GetDamage))
    (Actor|DestroyActor)))

(event EventBeginPlay
  (|CallParentFunction)
  (Utilities|Time|SetTimerbyEvent (delegate Custom|DetonateNearChar) 0.5 true))

(fn ConstructionScript
  (|CallParentFunction))