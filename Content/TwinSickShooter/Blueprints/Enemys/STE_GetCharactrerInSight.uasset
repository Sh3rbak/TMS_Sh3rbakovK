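; State Tree evaluator for enemy AI that supplies the player character as a target through AI perception.
; On tree start, it binds to the AI controller's perception component's target perception update event.
; Each update sets TargetChar to the player when that is the perceived actor and clears it for any other actor.
; The stimulus is not checked, so losing sight of the player still sets the target.
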(event EventTreeStart
  (bind _aicontroller (Variables|Context|GetAIController))
  (bind _returnvalue (Class|AIController|GetAIPerceptionComponent _aicontroller))
  (Utilities|IsValid _returnvalue
    (:Is%20Valid
      (EventDispatchers|BindEventtoOnTargetPerceptionUpdated _returnvalue (EventDispatchers|CreateEvent :!event STEGetCharactrerinSightAutoGenFunc)))))

(fn STEGetCharactrerinSightAutoGenFunc
  (params (Actor :type Actor%20Object%20Reference) (Stimulus :type AI%20Stimulus%20Structure))
  (bind _returnvalue (Game|GetPlayerCharacter 0))
  (if (== Actor _returnvalue)
    (bind _output_get (Variables|Output|SetTargetChar _returnvalue))
    (else
      (Variables|Output|SetTargetChar 0))))