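; Cube enemy for a twin-stick shooter, with a health component, a widget health bar and floating pawn movement.
; On BeginPlay it targets the first Character found and binds health changes to refresh the bar.
; Unwired chase logic turns it toward the target and moves it at the player, sphere-tracing ahead to rise over obstacles.
; Tick is empty, so that rotation and movement never run.
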(event Custom|OnHealthChange_Event
  (CallFunction|UpdateHealthBar))

(event EventBeginPlay
  (CallFunction|TargetPawnPlayer)
  (EventDispatchers|AssignOnHealthChange (Variables|Default|GetHealthComponentTSS) (delegate Custom|OnHealthChange_Event)))

(event EventTick
  (params (DeltaSeconds :type Float%20%28single-precision%29)))

(fn ConstructionScript)

(fn TargetPawnPlayer
  (bind _outactors (Actor|GetAllActorsOfClass "/Script/Engine.Character"))
  (if (Utilities|Array|IsValidIndex _outactors)
    (Variables|Default|SetTargetPawn (Utilities|Array|Get(acopy) _outactors))))

(fn InterpolationRotation
  (Variables|Default|GetTargetPawn
    (:then
      (Transformation|SetActorRotation (Math|Interpolation|RInterpTo (Transformation|GetActorRotation) (Math|Rotator|FindLookatRotation (Transformation|GetActorLocation) (Transformation|GetActorLocation (Variables|Default|GetTargetPawn))) (Utilities|Time|GetWorldDeltaSeconds) (Variables|Default|GetInterp%20Speed))))
    (:else)))

(fn UpdateHealthBar
  (bind _aswbp_tss_health_bar (Utilities|Casting|CastToWBP_TSS_HealthBar (UserInterface|GetWidget (Variables|Default|GetWidget))))
  (Progress|SetPercent (Variables|/Game/TwinSickShooter/Widget/WBP_TSS_HealthBar.WBP_TSS_HealthBar_C|GetHealthBar _aswbp_tss_health_bar) (Variables|/Game/TwinSickShooter/Blueprints/Component/HealthComponentTSS.HealthComponentTSS_C|GetHealthPercent (Variables|Default|GetHealthComponentTSS))))

(fn GetHorizontalDirecion
  (bind _returnvalue (Transformation|GetActorLocation))
  (bind _returnvalue_2 (Game|GetPlayerCharacter 0))
  (bind _returnvalue_3 (Transformation|GetActorLocation _returnvalue_2))
  (bind _returnvalue_4 (- _returnvalue_3 _returnvalue))
  (Utilities|IsValid _returnvalue_2
    (:Is%20Valid
      (return (Math|Vector|Normalize (Math|Vector|MakeVector (.x _returnvalue_4) (.y _returnvalue_4) 0.0))))))

(fn GetDirectiontoPlayer
  (bind _returnvalue (Game|GetPlayerCharacter 0))
  (Utilities|IsValid _returnvalue
    (:Is%20Valid
      (return (Math|Vector|Normalize (- (Transformation|GetActorLocation _returnvalue) (Transformation|GetActorLocation)))))))

(fn GetVireticalDirectionUp
  (return (Math|Vector|Normalize (+ (CallFunction|GetHorizontalDirecion) (* (Transformation|GetActorUpVector) (Variables|Default|GetOffsetUp))))))

(fn GetSphereTraceforObstacles
  (bind _returnvalue (Transformation|GetActorLocation))
  (return _returnvalue (+ _returnvalue (* (CallFunction|GetHorizontalDirecion) 1.5e+02))))