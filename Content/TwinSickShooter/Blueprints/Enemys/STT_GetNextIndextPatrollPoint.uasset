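; StateTree task that picks the next patrol point for a twin-stick shooter enemy.
; On entering the state it casts the owning pawn to BP_TSS_BaseEnemy and reads its target point list and current index, resetting a negative index to zero.
; It stores the selected point in TargetPoint, then advances the enemy's index with modulo wrap-around, so the patrol loops through the list.
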(event EventLatentEnterState
  (params (Transition :type State%20Tree%20Transition%20Result%20Structure%20%28by%20ref%29))
  (bind _asbp_tss_base_enemy (Utilities|Casting|CastToBP_TSS_BaseEnemy (Variables|Context|GetOwnPawn)))
  (Variables|Default|SetTarget%20Points (Variables|/Game/TwinSickShooter/Blueprints/Enemys/BP_TSS_BaseEnemy.BP_TSS_BaseEnemy_C|GetTargetPoints _asbp_tss_base_enemy))
  (Variables|Default|SetIndex%20Target%20Point (Variables|/Game/TwinSickShooter/Blueprints/Enemys/BP_TSS_BaseEnemy.BP_TSS_BaseEnemy_C|GetIndexTargetPoint _asbp_tss_base_enemy))
  (if (>= (Variables|Default|GetIndex%20Target%20Point) 0)
    _
    (else
      (Variables|Default|SetIndex%20Target%20Point 0)))
  (Variables|Output|SetTargetPoint (Utilities|Array|Get(acopy) (Variables|Default|GetTarget%20Points) (Math|Integer|%(Integer) (Variables|Default|GetIndex%20Target%20Point) (Utilities|Array|Length (Variables|Default|GetTarget%20Points)))))
  (Variables|/Game/TwinSickShooter/Blueprints/Enemys/BP_TSS_BaseEnemy.BP_TSS_BaseEnemy_C|SetIndexTargetPoint _asbp_tss_base_enemy (Math|Integer|%(Integer) (+ (Variables|Default|GetIndex%20Target%20Point) 1) (Utilities|Array|Length (Variables|Default|GetTarget%20Points)))))